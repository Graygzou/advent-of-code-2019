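; Puzzle solver Blueprint (Day 11) that drives a hull-painting style robot from a comma-separated instruction program loaded from a file.
; Two input actions each initialize the program and robot, differing in starting color.
; Each loops ComputeOneStep, feeding its outputs to MoveRobot until the program reports completion.
; Part 1 then prints the painted-panel data and count, while Part 2 displays the registration identifier.
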(event `InputAction|Fire Part 1`
  (params (Key :type "Key Structure"))
  ;[1 1 1] Part 1
  (:`Pressed`
    (`self.Init` (`ReadWriteFile.SplitString` (`ReadWriteFile.FileLoadString` (`self.inputPath`)) ","))
    (`self.InitRobot` (0.0 1.0))
    (bind (_outputs _returnvalue) (`self.ComputeOneStep` 2 :!label _label))
    (if _returnvalue
      (bind (_keys _values _returnvalue_2) (`self.GetNumberPanelsPainted`))
      (for _array_element _values
        (`KismetSystemLibrary.PrintString` (`KismetStringLibrary.Conv_IntToString` _array_element)))
      (for _array_element_2 _keys
        (`KismetSystemLibrary.PrintString` (`KismetStringLibrary.Conv_Vector2dToString` _array_element_2)))
      (`KismetSystemLibrary.PrintString` (`KismetStringLibrary.Conv_IntToString` _returnvalue_2))
      (else
        (`self.MoveRobot` _outputs)
        (goto _label)))))

(event `InputAction|Fire Part 2`
  (params (Key :type "Key Structure"))
  ;[1 1 1] Part2
  (:`Pressed`
    (`self.Init` (`ReadWriteFile.SplitString` (`ReadWriteFile.FileLoadString` (`self.inputPath`)) ","))
    (`self.InitRobot` (0.0 1.0) (0.0 0.0) 1)
    (bind (_outputs _returnvalue) (`self.ComputeOneStep` 2 :!label _label_2))
    (if _returnvalue
      (`self.DisplayRegistrationIdentifier`)
      (else
        (`self.MoveRobot` _outputs)
        (goto _label_2)))))

(fn `UserConstructionScript`)