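; BP_Day3 solves a "Day 3" two-wire puzzle from a text input, triggered by the Fire Part 1 input action.
; It loads the file, splits it into lines, then splits the first line and the following one on commas into two wire direction arrays.
; Both arrays go to ComputeDay3, defined outside this graph, and its return value and step number are printed.
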(event `InputAction|Fire Part 1`
  (params (Key :type "Key Structure"))
  (:`Pressed`
    (`self.Day3Part1` (`ReadWriteFile.SplitString` (`ReadWriteFile.FileLoadString` (`self.dayInput`)) "\\n"))))

(fn `Day3Part1`
  (params (NewParam :type "Array of String"))
  (for (_array_element _array_index) NewParam
    (if (== _array_index 0)
      (bind _returnvalue (`ReadWriteFile.SplitString` _array_element ","))
      (set `self.FirstWireArray` _returnvalue)
      (else
        (set `self.SecondWireArray` _returnvalue))))
  (bind (_stepnumber _returnvalue_2) (`Day3.ComputeDay3` (`self.FirstWireArray`) (`self.SecondWireArray`)))
  (`KismetSystemLibrary.PrintString` (`KismetStringLibrary.Conv_IntToString` _returnvalue_2))
  (`KismetSystemLibrary.PrintString` (`KismetStringLibrary.Conv_IntToString` _stepnumber)))

(fn `UserConstructionScript`)