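; Day 11 puzzle solver Blueprint that runs a comma-separated instruction program from a text file to drive a hull-painting style robot.
; Fire Part 1 loops the computer in two-output steps, feeding each result to MoveRobot until it finishes, then prints the painted panels and their count.
; Fire Part 2 is only a test that runs the program on preset inputs and prints every output.
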(event `InputAction|Fire Part 2`
  (params (Key :type "Key Structure"))
  ;[1 1 1] Test
  (:`Pressed`
    (`Day11.Init` (`ReadWriteFile.SplitString` (`ReadWriteFile.FileLoadString` (`self.inputPath`)) ","))
    (bind _outputs (`Day11.ComputeOneStepWithInputs` (`self.NewVar_0`) 1000000000))
    (for _array_element _outputs
      (`KismetSystemLibrary.PrintString` (`KismetTextLibrary.Conv_TextToString` (`KismetTextLibrary.Conv_Int64ToText` _array_element))))))

(event `InputAction|Fire Part 1`
  (params (Key :type "Key Structure"))
  ;[1 1 1] Part 1
  (:`Pressed`
    (`Day11.Init` (`ReadWriteFile.SplitString` (`ReadWriteFile.FileLoadString` (`self.inputPath`)) ","))
    (`Day11.InitRobot` (0.0 1.0))
    (bind (_outputs _returnvalue) (`Day11.ComputeOneStep` 2 :!label _label))
    (if _returnvalue
      (bind (_keys _values _returnvalue_2) (`Day11.GetNumberPanelsPainted`))
      (for _array_element _values
        (`KismetSystemLibrary.PrintString` (`KismetStringLibrary.Conv_IntToString` _array_element)))
      (for _array_element_2 _keys
        (`KismetSystemLibrary.PrintString` (`KismetStringLibrary.Conv_Vector2dToString` _array_element_2)))
      (`KismetSystemLibrary.PrintString` (`KismetStringLibrary.Conv_IntToString` _returnvalue_2))
      (else
        (`Day11.MoveRobot` _outputs)
        (goto _label)))))

(fn `UserConstructionScript`)