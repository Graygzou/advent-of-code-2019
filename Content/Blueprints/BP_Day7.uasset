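; BP_Day7 is a Day 7 puzzle solver that searches for the right combination of values to run through a comma-separated program.
; Each trigger loads the input file, splits it on commas and passes it on with the starting input and current combination.
; The two Fire Part inputs print the Part 1 and Part 2 search results.
; The 3 key runs ComputeNCycle on the same data without printing its result.
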(event `InputAction|Fire Part 1`
  (params (Key :type "Key Structure"))
  (:`Pressed`
    (bind _returnvalue (`Day7.FindRightCombinaison` (`ReadWriteFile.SplitString` (`ReadWriteFile.FileLoadString` (`self.InputPath`)) ",") (`self.startingInput`) (`self.combinaison`)))
    (`KismetSystemLibrary.PrintString` (`KismetStringLibrary.Conv_IntToString` _returnvalue))))

(event `InputAction|Fire Part 2`
  (params (Key :type "Key Structure"))
  (:`Pressed`
    (bind _returnvalue (`Day7.FindRightCombinaisonPart2` (`ReadWriteFile.SplitString` (`ReadWriteFile.FileLoadString` (`self.InputPath`)) ",") (`self.startingInput`) (`self.combinaison`)))
    (`KismetSystemLibrary.PrintString` (`KismetStringLibrary.Conv_IntToString` _returnvalue))))

(event `Key|Three`
  (params (Key :type "Key Structure"))
  (:`Pressed`
    (`Day7.ComputeNCycle` (`ReadWriteFile.SplitString` (`ReadWriteFile.FileLoadString` (`self.InputPath`)) ",") (`self.combinaison`) (`self.startingInput`))))

(fn `UserConstructionScript`)