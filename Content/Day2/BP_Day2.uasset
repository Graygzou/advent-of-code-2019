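; Blueprint that solves part 1 of a Day 2 puzzle that runs comma-separated opcode programs, triggered by the Fire Part 1 input action.
; Day2Part1 runs four hardcoded test programs, then the program loaded from the InputPath file.
; Each is split on commas and passed to ComputeDay2Part1, which calls Compute and prints the array as a joined string.
; The PrintOpcode debug loops in the event graph are disconnected.
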(event `InputAction|Fire Part 1`
  (params (Key :type "Key Structure"))
  (:`Pressed`
    (`self.Day2Part1` (`self.inputPath`))))

(event `InputAction|Fire Part 2`
  (params (Key :type "Key Structure")))

(fn `ComputeDay2Part1`
  (params (NewParam :type "Array of String"))
  (locals (inputArray :type "Array of String") (res :type String))
  (bind _output_get (set `local.inputArray` NewParam))
  (`Day2.Compute` _output_get (`self.input`))
  (for _array_element (`local.inputArray`)
    (set `local.res` (`KismetStringLibrary.Concat_StrStr` (`local.res`) " , " _array_element)))
  (`KismetSystemLibrary.PrintString` (`local.res`)))

(fn `Day2part1`
  (params (inputFilePath :type String))
  ;[1 1 1] Unit tests
  (`self.ComputeDay2Part1` (`ReadWriteFile.SplitString` "1,0,0,0,99" ","))
  (`self.ComputeDay2Part1` (`ReadWriteFile.SplitString` "2,3,0,3,99" ","))
  (`self.ComputeDay2Part1` (`ReadWriteFile.SplitString` "2,4,4,5,99,0" ","))
  (`self.ComputeDay2Part1` (`ReadWriteFile.SplitString` "1,1,1,4,99,5,6,0,99" ","))
  (`self.ComputeDay2Part1` (`ReadWriteFile.SplitString` (`ReadWriteFile.FileLoadString` inputFilePath) ",")))

(fn `UserConstructionScript`)