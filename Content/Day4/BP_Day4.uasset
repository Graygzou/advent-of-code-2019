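; BP_Day4 is a Blueprint that runs part 1 of a "Day 4" puzzle from a fire input and prints the answer.
; The first press splits the Input string at a hyphen into integer lower and upper bounds, or prints the failed split result.
; Day4part1 passes the bounds to ComputeDay4, whose logic lives outside these graphs, and prints what it returns.
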(event `InputAction|Fire Part 1`
  (params (Key :type "Key Structure"))
  (bind (_lefts _rights _returnvalue) (`KismetStringLibrary.Split` (`self.input`) "-"))
  (:`Pressed`
    (`/Engine/EditorBlueprintResources/StandardMacros.DoOnce` false
      (:`Completed`
        (if _returnvalue
          (`self.day4part1` (`KismetStringLibrary.Conv_StringToInt` _lefts) (`KismetStringLibrary.Conv_StringToInt` _rights))
          (else
            (`KismetSystemLibrary.PrintString` (`KismetStringLibrary.Conv_BoolToString` _returnvalue))))))))

(fn `day4part1`
  (params (lowerBound :type Integer) (upperBound :type Integer))
  (bind _returnvalue (`Day4.ComputeDay4` lowerBound upperBound))
  (`KismetSystemLibrary.PrintString` (`KismetStringLibrary.Conv_IntToString` _returnvalue)))

(fn `UserConstructionScript`)